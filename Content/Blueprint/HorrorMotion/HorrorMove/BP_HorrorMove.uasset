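; Horror scare actor that plays a HorrorScenario list of visibility, move and rotate steps when NextHorrorTrigger fires and ActiveHorror is set.
; Steps use latent Delays inside the loop, which do not pause iteration, then set shared targets and interp speed.
; Tick eases toward those targets with VInterpTo and RInterpTo, printing the interpolated location.
; Unless IsInfinity is set, the actor destroys itself after an EndTime delay.
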(event EventBeginPlay
  (|CallParentFunction) ; 지금 이 노드는 비활성 상태입니다. \n핀을 끌어서 다른 노드를 연결하면 활성화됩니다.
)

(event Collision|EventActorBeginOverlap
  (params (OtherActor :type Actor%20Object%20Reference))
  (|CallParentFunction OtherActor) ; 지금 이 노드는 비활성 상태입니다. \n핀을 끌어서 다른 노드를 연결하면 활성화됩니다.
)

(event EventTick
  (params (DeltaSeconds :type Float%20%28single-precision%29))
  (bind _returnvalue (Transformation|GetActorLocation))
  (bind _array_element_interp_speed (Variables|Default|GetArray%20Element%20Interp%20Speed))
  (bind _array_element_location (Variables|Default|GetArray%20Element%20Location))
  (bind _returnvalue_2 (Math|Interpolation|VInterpTo _returnvalue _array_element_location DeltaSeconds _array_element_interp_speed))
  (|CallParentFunction DeltaSeconds)
  (Utilities|FlowControl|Sequence
    (:then_0
      (if (Variables|Default|GetMoveLocation)
        (Transformation|SetActorLocation _returnvalue_2 false false)
        (Development|PrintString (Utilities|String|ToString(Vector) _returnvalue_2))))
    (:then_1
      (if (Variables|Default|GetMoveRotation)
        (Transformation|SetActorRotation (Math|Interpolation|RInterpTo (Transformation|GetActorRotation) (Variables|Default|GetArray%20Element%20Rotation) DeltaSeconds _array_element_interp_speed))))))

(event EventNextHorrorTrigger
  (params (Trigger :type Boolean))
  (|CallParentFunction Trigger)
  (if (Variables|Default|GetActiveHorror)
    (for _array_element (Variables|Default|GetHorrorScenario)
      (switch Utilities|FlowControl|Switch|SwitchonE_HorrorMoveLabel (.horrormovelabel _array_element)
        (:NewEnumerator3
          (Utilities|FlowControl|Delay (.time _array_element))
          (Rendering|SetVisibility (Variables|Default|GetDefaultSceneRoot) (.bvisible _array_element) true))
        (:NewEnumerator1
          (Utilities|FlowControl|Delay (.time _array_element))
          (Variables|Default|SetArray%20Element%20Location (.movelocation _array_element))
          (Variables|Default|SetMoveLocation true)
          (Variables|Default|SetArray%20Element%20Interp%20Speed (.interpspeed _array_element) :!label _label))
        (:NewEnumerator2
          (Utilities|FlowControl|Delay (.time _array_element))
          (Variables|Default|SetArray%20Element%20Rotation (.moverotation _array_element))
          (Variables|Default|SetMoveRotation true)
          (goto _label)))
      (if (not (Variables|Default|GetbIsInfinity))
        (Utilities|FlowControl|Delay (.endtime _array_element))
        (Actor|DestroyActor)))))

(fn ConstructionScript
  (|CallParentFunction))