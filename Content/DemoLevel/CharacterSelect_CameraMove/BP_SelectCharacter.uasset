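; Selectable character actor for a character selection demo that moves the player's view to this character's camera.
; CharacterSelect blends the first player controller's view target to the owner of Camera over CameraBlendTime, locking the outgoing view during the transition.
; IsCharacterSelect reports whether a given name matches CharacterName.
; The event graph and construction script are empty, so both functions rely on outside callers.
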(event EventBeginPlay)

(event Collision|EventActorBeginOverlap
  (params (OtherActor :type Actor%20Object%20Reference)))

(event EventTick
  (params (DeltaSeconds :type Float%20%28single-precision%29)))

(fn ConstructionScript)

(fn CharacterSelect
  (Game|Player|SetViewTargetwithBlend (Game|GetPlayerController 0) (Components|GetOwner (Variables|Default|GetCamera)) (Variables|Default|GetCameraBlend%20Time) "VTBlend_Linear" 0.0 true))

(fn IsCharacterSelect
  (params (CharacterName :type ECharacterSelectName%20Enum :default "NewEnumerator0"))
  (if (Utilities|Enum|Equal(Enum) CharacterName (Variables|Default|GetCharacterName))
    (return true)
    (else
      (return false))))