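; Manager actor for a demo character-select screen, linking the selection UI to the selectable characters in the level.
; On BeginPlay it creates and displays the WBP_SelectCharacter_CameraMove widget and gathers all BP_SelectCharacter actors.
; It binds the widget's button click to an event that finds the first character matching the clicked name and calls CharacterSelect on it.
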(event Custom|SelectCharacterButtonClick_Event
  (params (CharacterName :type ECharacterSelectName%20Enum :default "NewEnumerator0"))
  ;[0.15 0.15 0.15 0.5] 동일한 이름 찾기
  (bind _array_element (Utilities|Array|ForEachLoopwithBreak (Variables|Default|GetBP_SelectCharacterArr_Ref) :!label _label)
    (:LoopBody
      (if (Default|IsCharacterSelect _array_element CharacterName)
        (Default|CharacterSelect _array_element)
        (goto _label Break)))))

(event EventBeginPlay
  ;[0.15 0.15 0.15 0.5] 위젯 생성 및 드로우
  (bind _returnvalue (UserInterface|CreateWidget "/Game/DemoLevel/CharacterSelect_CameraMove/WBP_SelectCharacter_CameraMove.WBP_SelectCharacter_CameraMove_C" (Game|GetPlayerController 0)))
  (bind _output_get (Variables|Default|SetWBP_SelectCharacterWidgetRef _returnvalue))
  (UserInterface|Viewport|AddtoViewport _output_get 0)
  ;[0.15 0.15 0.15 0.5] 캐릭터 수집
  (bind _outactors (Actor|GetAllActorsOfClass "/Game/DemoLevel/CharacterSelect_CameraMove/BP_SelectCharacter.BP_SelectCharacter_C"))
  (Variables|Default|SetBP_SelectCharacterArr_Ref _outactors)
  (EventDispatchers|AssignSelectCharacterButtonClick (Variables|Default|GetWBP_SelectCharacterWidgetRef) (delegate Custom|SelectCharacterButtonClick_Event)))

(fn ConstructionScript)